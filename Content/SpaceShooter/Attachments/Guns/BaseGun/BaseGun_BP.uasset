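; BaseGun_BP is a space shooter gun attachment that fires projectiles when its owner's fire-guns dispatcher triggers.
; On BeginPlay it asks the GameState's PoolMaster to pool projectiles in proportion to rate of fire (ROF).
; Firing takes a pooled projectile at ProjectileSpawn, passes yaw through GetRandomYaw and sets the Instigator.
; Capped upgrades raise ROF and accuracy; the reusable spawn-particle effect is never called.
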(event `self.ReceiveBeginPlay`
  (bind _asgame_state_bp (cast `/Game/SpaceShooter/GameState_BP` (`GameplayStatics.GetGameState`)))
  (bind _master (`/Game/SpaceShooter/GameState_BP.GetPoolMaster` _asgame_state_bp))
  (bind _output_get (set `self.PoolMasterPtr` _master))
  (`PoolMaster.RequestAddition` _output_get (`self.Projectile`) (`KismetMathLibrary.FCeil` (* (`self.ROF`) 5.0))))

(event `self.AttachmentBind`
  (params (Owner :type "/Game/SpaceShooter/Ships/BaseShip_BP Object Reference"))
  (add `/Game/SpaceShooter/Ships/BaseShip_BP.FireGunsDispatch` Owner (delegate `FireGun`)))

(event `FireGun`
  (bind (_returnvalue_location _returnvalue_rotation _returnvalue_scale) (`KismetMathLibrary.BreakTransform` (`SceneComponent.K2_GetComponentToWorld` (`self.ProjectileSpawn`))))
  ;[1 1 1] @TODO : Implement spawning of projectile
  (bind _objectspawned (`PoolMaster.SpawnObject` (`self.PoolMasterPtr`) (`self.Projectile`) (`KismetMathLibrary.MakeTransform` _returnvalue_location (`KismetMathLibrary.MakeRotator` (.roll _returnvalue_rotation) (.pitch _returnvalue_rotation) (`self.GetRandomYaw` (.yaw _returnvalue_rotation))) _returnvalue_scale) self))
  (`/Engine/EditorBlueprintResources/StandardMacros.IsValid` _objectspawned
    (:`Is Valid`
      (set `Actor.Instigator` (`self.GetInstigator`) _objectspawned))))

(event `UpgradeROF`
  (bind _returnvalue (+ (`self.ROF`) (`self.ROFUpgradeAmount`)))
  (if (not (> (`self.MaxROF`) _returnvalue))
    (set `self.CanUpgradeROF` false))
  (set `self.ROF` (`KismetMathLibrary.FClamp` _returnvalue 0.5 (`self.MaxROF`))))

(event `UpgradeAccuracy`
  (bind _returnvalue (+ (`self.Accuracy`) (`self.AccuracyUpgradeAmount`)))
  (if (not (> (`self.MaxAccuracy`) _returnvalue))
    (set `self.CanUpgradeAccuracy` false))
  (set `self.Accuracy` (`KismetMathLibrary.FClamp` _returnvalue 0.0 (`self.MaxAccuracy`))))

(fn `FirePartSpawn`
  (bind _spawnpartsys (`self.SpawnPartSys`))
  (`/Engine/EditorBlueprintResources/StandardMacros.IsValid` (`self.SpawnPartSys`)
    (:`Is Valid`
      (`SceneComponent.K2_SetWorldLocation` _spawnpartsys (`self.K2_GetActorLocation`) false true)
      (`SceneComponent.K2_SetWorldRotation` _spawnpartsys (`self.K2_GetActorRotation`) false false)
      (`NiagaraComponent.ResetSystem` _spawnpartsys))
    (:`Is Not Valid`
      (bind _returnvalue (`NiagaraFunctionLibrary.SpawnSystemAtLocation` (`self.SpawnParticles`) (`self.K2_GetActorLocation`) (`self.K2_GetActorRotation`) false))
      (set `self.SpawnPartSys` _returnvalue))))

(fn `GetCanUpgradeAccuracy`
  (returns (`Can it?` :type Boolean))
  (return (`self.CanUpgradeAccuracy`)))

(fn `GetCanUpgradeROF`
  (returns (`Can it?` :type Boolean))
  (return (`self.CanUpgradeROF`)))

(fn `UserConstructionScript`)