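; BaseGunPreview_BP is a preview actor that renders a gun for display in UI in the space shooter.
; Its construction script creates a render target, assigns it to a SceneCaptureComponent2D, and feeds it into a dynamic instance of a UI material.
; Tick slowly spins the PivotPoint around yaw for a turntable view.
; GetUIRenderMaterial returns the dynamic material so UI can show the live capture.
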(event `self.ReceiveTick`
  (params (DeltaSeconds :type "Float (single-precision)"))
  (`SceneComponent.K2_AddLocalRotation` (`self.PivotPoint`) (`KismetMathLibrary.MakeRotator` 0.0 0.0 (* DeltaSeconds -10.0)) false false))

(fn `GetUIRenderMaterial`
  (returns (`UI Material` :type "MaterialInstanceDynamic Object Reference"))
  (return (`self.UIMaterialDynamic`)))

(fn `UserConstructionScript`
  (bind _returnvalue (`KismetRenderingLibrary.CreateRenderTarget2D` 512))
  (bind _output_get (set `self.RT` _returnvalue))
  (set `SceneCaptureComponent2D.TextureTarget` _output_get (`self.SceneCaptureComponent2D`))
  (bind _returnvalue_2 (`KismetMaterialLibrary.CreateDynamicMaterialInstance` (`self.UIMaterialStatic`)))
  (bind _output_get_2 (set `self.UIMaterialDynamic` _returnvalue_2))
  (`MaterialInstanceDynamic.SetTextureParameterValue` _output_get_2 "RenderTarget" (`self.RT`)))