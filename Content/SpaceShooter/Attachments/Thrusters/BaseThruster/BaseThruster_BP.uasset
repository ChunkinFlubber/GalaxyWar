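; BaseThruster_BP is the base thruster attachment for the space shooter, tracking whether the thruster is firing.
; When bound to an owner, it subscribes its fire and stop events to the owner's thruster dispatchers.
; Those events only toggle the IsThrusting flag, guarded against redundant changes, with no force or effects applied in this graph.
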(event `self.AttachmentBind`
  (params (Owner :type "/Game/SpaceShooter/Ships/BaseShip_BP Object Reference"))
  (add `/Game/SpaceShooter/Ships/BaseShip_BP.FireThrustersDispatch` Owner (delegate `FireThruster`))
  (add `/Game/SpaceShooter/Ships/BaseShip_BP.StopThrustersDispatch` Owner (delegate `StopThruster`)))

(event `StopThruster`
  (if (`self.IsThrusting`)
    (set `self.IsThrusting` false)))

(event `FireThruster`
  (if (not (`self.IsThrusting`))
    (set `self.IsThrusting` true)))

(fn `UserConstructionScript`
  (`parent.UserConstructionScript`))