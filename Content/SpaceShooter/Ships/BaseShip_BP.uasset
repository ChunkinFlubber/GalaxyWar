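; BaseShip_BP is the base ship Blueprint for the space shooter, handling damage and destruction.
; On BeginPlay it binds to its own any-damage event and accepts only DefaultDamageType damage, which it subtracts from Health.
; Each hit fires a health-changed dispatcher, then either a destroyed dispatcher at zero health or below, or the damage type's DebuffFunction, letting damage types carry their own debuffs.
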(event `self.ReceiveBeginPlay`
  (add `self.OnTakeAnyDamage` (delegate `TakeDamage`)))

(event `TakeDamage` :!signature `self.OnTakeAnyDamage`
  (params (DamagedActor :type "Actor Object Reference") (Damage :type "Float (double-precision)") (DamageType :type "DamageType Object Reference") (InstigatedBy :type "Controller Object Reference") (DamageCauser :type "Actor Object Reference"))
  (bind _asdefault_damage_type (cast `/Game/SpaceShooter/Attachments/Guns/DefaultDamageType` DamageType))
  (set `self.Health` (- (`self.Health`) Damage))
  (`self.HealthChangedDispatch`)
  (if (<= (`self.Health`) 0.0)
    (`self.ShipDestroyedDispatch`)
    (else
      (`/Game/SpaceShooter/Attachments/Guns/DefaultDamageType.DebuffFunction` _asdefault_damage_type))))

(fn `UserConstructionScript`)