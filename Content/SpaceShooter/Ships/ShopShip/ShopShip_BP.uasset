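; Shop ship in the space shooter that lets the player open a shop menu when nearby.
; Overlapping its InteractionSpace shows an enter-shop popup and binds shop entry to the player pawn's interact event, undone on leaving.
; Entering swaps the popup for the shop menu with UI-only input and mouse cursor, while PlayerExitShop reverses this.
; Both widgets are created lazily and reused.
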(event `self.ReceiveBeginPlay`
  (bind _asplayer_pawn_bp (cast `/Game/SpaceShooter/Ships/PlayerShips/PlayerPawn_BP` (`GameplayStatics.GetPlayerPawn` 0)))
  (set `self.PlayerPawn` _asplayer_pawn_bp)
  (set `self.PlayerController` (`GameplayStatics.GetPlayerController` 0)))

(event `PlayerFar`
  (`/Engine/EditorBlueprintResources/StandardMacros.IsValid` (`self.ShopPopupWidget`)
    (:`Is Valid`
      (`Widget.RemoveFromParent` (`self.ShopPopupWidget`)))))

(event `PlayerClose`
  (`/Engine/EditorBlueprintResources/StandardMacros.IsValid` (`self.ShopPopupWidget`)
    (:`Is Valid`
      _)
    (:`Is Not Valid`
      (bind _returnvalue (`|CreateWidget` "/Game/SpaceShooter/UI/Shop/EnterShopPopupWidget.EnterShopPopupWidget_C" (`self.PlayerController`)))
      (bind _output_get (set `self.ShopPopupWidget` _returnvalue))))
  (`UserWidget.AddToViewport` _output_get 0))

(event `PlayerEnterShop`
  (`/Engine/EditorBlueprintResources/StandardMacros.IsValid` (`self.MainShopWidget`)
    (:`Is Valid`
      _)
    (:`Is Not Valid`
      (bind _returnvalue (`|CreateWidget` "/Game/SpaceShooter/UI/Shop/ShopMenuWidget.ShopMenuWidget_C" (`self.PlayerController`)))
      (bind _output_get (set `self.MainShopWidget` _returnvalue))))
  (`UserWidget.AddToViewport` _output_get 0)
  (`WidgetBlueprintLibrary.SetInputMode_UIOnlyEx` (`self.PlayerController`) _output_get)
  (set `PlayerController.bShowMouseCursor` true (`self.PlayerController`))
  (`Widget.RemoveFromParent` (`self.ShopPopupWidget`)))

(event `PlayerExitShop`
  (`/Engine/EditorBlueprintResources/StandardMacros.IsValid` (`self.MainShopWidget`)
    (:`Is Valid`
      (`Widget.RemoveFromParent` (`self.MainShopWidget`))
      (`WidgetBlueprintLibrary.SetInputMode_GameOnly` (`self.PlayerController`))
      (set `PlayerController.bShowMouseCursor` false (`self.PlayerController`))
      (`UserWidget.AddToViewport` (`self.ShopPopupWidget`) 0))))

(event `self.InteractionSpace.OnComponentBeginOverlap`
  (params (OverlappedComponent :type "PrimitiveComponent Object Reference") (OtherActor :type "Actor Object Reference") (OtherComp :type "PrimitiveComponent Object Reference") (OtherBodyIndex :type Integer) (bFromSweep :type Boolean) (SweepResult :type "HitResult Structure (by ref)"))
  (if (== OtherActor (`self.PlayerPawn`))
    (`self.PlayerClose`)
    (add `/Game/SpaceShooter/Ships/PlayerShips/PlayerPawn_BP.Interacted` (`self.PlayerPawn`) (delegate `PlayerEnterShop`))))

(event `self.InteractionSpace.OnComponentEndOverlap`
  (params (OverlappedComponent :type "PrimitiveComponent Object Reference") (OtherActor :type "Actor Object Reference") (OtherComp :type "PrimitiveComponent Object Reference") (OtherBodyIndex :type Integer))
  (if (== OtherActor (`self.PlayerPawn`))
    (`self.PlayerFar`)
    (remove `/Game/SpaceShooter/Ships/PlayerShips/PlayerPawn_BP.Interacted` (`self.PlayerPawn`) (delegate `PlayerEnterShop`))))

(fn `UserConstructionScript`)