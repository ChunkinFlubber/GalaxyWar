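; Base projectile for the space shooter, built for reuse through its parent's ActorSpawned and DisableActor events.
; Spawning launches it along local forward and starts a lifetime timer that calls DisableActor.
; Overlapping any non-owner actor applies damage and disables it.
; Disabling with a live timer clears it, deactivates movement and mesh, and plays a death particle system that is created once, then moved and reset.
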(event `self.ReceiveActorBeginOverlap`
  (params (OtherActor :type "Actor Object Reference"))
  (if (!= OtherActor (`self.GetOwner`))
    (`GameplayStatics.ApplyDamage` OtherActor (`self.ProjectileDamage`) null self "/Game/SpaceShooter/Attachments/Guns/DefaultDamageType.DefaultDamageType_C")
    (`self.DisableActor`)))

(event `self.DisableActor`
  (bind _lifetimer (`self.LifeTimer`))
  (`parent.DisableActor`)
  (if (`KismetSystemLibrary.K2_TimerExistsHandle` _lifetimer)
    (`KismetSystemLibrary.K2_ClearAndInvalidateTimerHandle` _lifetimer)
    (`ActorComponent.Deactivate` (`self.ProjectileMovement`))
    (`ActorComponent.Deactivate` (`self.BulletMesh`))
    (`self.DeathParticleSpawn`)))

(event `self.ActorSpawned`
  (`parent.ActorSpawned`)
  (`ProjectileMovementComponent.SetVelocityInLocalSpace` (`self.ProjectileMovement`) (1500.0 0.0 0.0))
  (bind _returnvalue (`KismetSystemLibrary.K2_SetTimerDelegate` (delegate `self.DisableActor`) 5.0))
  (set `self.LifeTimer` _returnvalue)
  (`ActorComponent.Activate` (`self.ProjectileMovement`) false)
  (`ActorComponent.Activate` (`self.BulletMesh`) false))

(fn `DeathParticleSpawn`
  (bind _deathpartsys (`self.DeathPartSys`))
  (`/Engine/EditorBlueprintResources/StandardMacros.IsValid` (`self.DeathPartSys`)
    (:`Is Valid`
      (`SceneComponent.K2_SetWorldLocation` _deathpartsys (`self.K2_GetActorLocation`) false true)
      (`NiagaraComponent.ResetSystem` _deathpartsys))
    (:`Is Not Valid`
      (bind _returnvalue (`NiagaraFunctionLibrary.SpawnSystemAtLocation` (`self.DeathParticles`) (`self.K2_GetActorLocation`) (struct) false))
      (set `self.DeathPartSys` _returnvalue))))

(fn `UserConstructionScript`)